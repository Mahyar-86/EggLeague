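; BP_EggJa is an egg receptacle actor that keeps a count of the eggs currently inside its Box trigger.
; On BeginPlay, the Wich variable selects one of two goblin enemy materials for its static mesh components.
; Box begin and end overlaps raise and lower the Eggs counter for actors tagged "Egg".
; Nothing in this Blueprint reads the counter.
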(event OnComponentBeginOverlap(Box)
  (params (OverlappedComponent :type Primitive%20Component%20Object%20Reference) (OtherActor :type Actor%20Object%20Reference) (OtherComp :type Primitive%20Component%20Object%20Reference) (OtherBodyIndex :type Integer) (bFromSweep :type Boolean) (SweepResult :type Hit%20Result%20Structure%20%28by%20ref%29))
  (if (Actor|ActorHasTag OtherActor "Egg")
    (Math|Integer|IncrementInt (Variables|Default|GetEggs))))

(event OnComponentEndOverlap(Box)
  (params (OverlappedComponent :type Primitive%20Component%20Object%20Reference) (OtherActor :type Actor%20Object%20Reference) (OtherComp :type Primitive%20Component%20Object%20Reference) (OtherBodyIndex :type Integer))
  (if (Actor|ActorHasTag OtherActor "Egg")
    (Math|Integer|DecrementInt (Variables|Default|GetEggs))))

(event EventBeginPlay
  (bind _staticmesh (Variables|Default|GetStaticMesh))
  (if (== (Variables|Default|GetWich) 0)
    (Rendering|Material|SetMaterial _staticmesh 0 "/Game/UndeadPack/EnemyGoblin/Materials/M_EnemyGoblin_01.M_EnemyGoblin_01")
    (else
      (Rendering|Material|SetMaterial _staticmesh 0 "/Game/ThirdPerson/Blueprints/EnemyGoblin/Materials/MI_EnemyGoblin_02.MI_EnemyGoblin_02"))))

(event Collision|EventActorBeginOverlap
  (params (OtherActor :type Actor%20Object%20Reference)))

(fn ConstructionScript)